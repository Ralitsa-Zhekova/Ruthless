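; Spell actor that acts as a hit volume, killing AI_BP characters it overlaps.
; Its sphere, scaled by CollisionScale at construction, calls CallDie and TellServerIGotHit on AI hit, then spawns an explosion and destroys the spell.
; Other overlaps also explode and destroy it; the player-character check compares the failed cast result, so it does not exclude the player.
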(event `self.Sphere.OnComponentBeginOverlap`
  (params (OverlappedComponent :type "PrimitiveComponent Object Reference") (OtherActor :type "Actor Object Reference") (OtherComp :type "PrimitiveComponent Object Reference") (OtherBodyIndex :type Integer) (bFromSweep :type Boolean) (SweepResult :type "HitResult Structure (by ref)"))
  (bind _asai_bp (cast `/Game/Blueprints/Characters/AI_BP` OtherActor)
    (:`then`
      (`/Game/Blueprints/Characters/AI_BP.Die` _asai_bp)
      (`/Game/Blueprints/Characters/AI_BP.TellServerIGotHit` _asai_bp)
      (`GameplayStatics.SpawnEmitterAtLocation` "/Game/Luos8Elements/Particles/Light/P_HitExplo.P_HitExplo" (`self.K2_GetActorLocation`))
      (`self.K2_DestroyActor`))
    (:`CastFailed`
      (if (not (== _asai_bp (`GameplayStatics.GetPlayerCharacter` 0)))
        (`GameplayStatics.SpawnEmitterAtLocation` "/Game/Luos8Elements/Particles/Light/P_HitExplo.P_HitExplo" (`self.K2_GetActorLocation`))
        (`self.K2_DestroyActor`)))))

(fn `UserConstructionScript`
  (`SceneComponent.SetWorldScale3D` (`self.Sphere`) (`self.Collision Scale`)))